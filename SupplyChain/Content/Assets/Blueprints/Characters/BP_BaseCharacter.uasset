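; Base player character with a physics pick-up and drop system tied to quest objective progress.
; An input toggle traces from the camera and grabs simulating components with a physics handle, which Tick keeps at HoldPoint until released.
; Tick also advances ObjectiveStatus and fires quest calls 1.2 or 2.2 when HasObject is valid at the matching stage.
; HasObject is never cleared on drop, so it records the last grabbed component.
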(event Custom|PickingUp
  (bind _playercam (Variables|Default|GetplayerCam))
  (bind _returnvalue (Transformation|GetWorldLocation _playercam))
  ;[1 1 1] Pick-up System
  (bind (_outhit _returnvalue_2) (Collision|LineTraceByChannel _returnvalue (+ _returnvalue (* (Math|Vector|GetForwardVector _playercam) 3e+02)) "TraceTypeQuery2" false 0 "ForDuration" true "(R=1.000000,G=0.000000,B=0.000000,A=0.000000)" "(R=0.000000,G=1.000000,B=0.000000,A=0.000000)" 0.0))
  (if _returnvalue_2
    (if (Physics|IsSimulatingPhysics (.HitComponent (Collision|BreakHitResult _outhit)) "None")
      (Physics|Components|PhysicsHandle|GrabComponentatLocationwithRotation (Variables|Default|GetObjectGrabber) (.HitComponent (Collision|BreakHitResult _outhit)) "None" (Transformation|GetWorldLocation (.HitComponent (Collision|BreakHitResult _outhit))) "0, 0, 0")
      (Variables|Default|SetHolding? true)
      (Variables|Default|SetHasObject (.HitComponent (Collision|BreakHitResult _outhit))))
    (else
      (Development|PrintString "1"))))

(event Custom|Dropping
  ;[1 1 1] Pick-up System
  (Physics|Components|PhysicsHandle|ReleaseComponent (Variables|Default|GetObjectGrabber))
  (Variables|Default|SetHolding? false))

(event EventBeginPlay
  (Variables|Default|SetObjectiveStatus "NewEnumerator0"))

(event Collision|EventActorBeginOverlap
  (params (OtherActor :type Actor%20Object%20Reference)))

(event EventTick
  (params (DeltaSeconds :type Float%20%28single-precision%29))
  (Utilities|FlowControl|Sequence
    (:then_0
      ;[1 1 1] Objective 1.1
      (if (and (Utilities|IsValid (Variables|Default|GetHasObject)) (Utilities|Enum|Equal(Enum) (Variables|Default|GetObjectiveStatus) "NewEnumerator0"))
        (Variables|Default|SetObjectiveStatus "NewEnumerator1")
        (Default|CallQuestCall1-2)))
    (:then_1
      ;[1 1 1] Objective 1.1
      (if (and (Utilities|IsValid (Variables|Default|GetHasObject)) (Utilities|Enum|Equal(Enum) (Variables|Default|GetObjectiveStatus) "NewEnumerator2"))
        (Variables|Default|SetObjectiveStatus "NewEnumerator3")
        (Default|CallQuestCall2-2)))
    (:then_2
      ;[1 1 1] Pick-up System
      (if (Variables|Default|GetHolding?)
        (Physics|Components|PhysicsHandle|SetTargetLocation (Variables|Default|GetObjectGrabber) (Transformation|GetWorldLocation (Variables|Default|GetHoldPoint)))))))

(event Input|ActionEvents|InputActionPickUp&Drop
  (params (Key :type Key%20Structure :default "None"))
  ;[1 1 1] Pick-up System
  (:Pressed
    (if (Variables|Default|GetHolding?)
      (CallFunction|Dropping)
      (else
        (CallFunction|PickingUp)))))

(fn ConstructionScript)